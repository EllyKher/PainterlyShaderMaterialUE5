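; Demo room actor for a painterly outer rim erosion effect, built as stacked copies of one instanced static mesh.
; The construction script adds four instances at the component's relative transform, intended as a diffuse layer, an eroded outer rim and two outline layers.
; Per-instance custom data tags the rim and outline layers, while the diffuse instance keeps its default and the event graph has no logic.
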(fn `UserConstructionScript`
  (bind _returnvalue (`SceneComponent.GetRelativeTransform` (`self.InstancedStaticMesh`)))
  ; Diffuse
  (`InstancedStaticMeshComponent.AddInstance` (`self.InstancedStaticMesh`) _returnvalue false)
  ; Outer Eroded Rim
  (bind _returnvalue_2 (`InstancedStaticMeshComponent.AddInstance` (`self.InstancedStaticMesh`) _returnvalue false))
  (`InstancedStaticMeshComponent.SetCustomDataValue` (`self.InstancedStaticMesh`) _returnvalue_2 0 1.0 false)
  ; Outlines
  (bind _returnvalue_3 (`InstancedStaticMeshComponent.AddInstance` (`self.InstancedStaticMesh`) _returnvalue false))
  (`InstancedStaticMeshComponent.SetCustomDataValue` (`self.InstancedStaticMesh`) _returnvalue_3 0 2.0 false)
  (bind _returnvalue_4 (`InstancedStaticMeshComponent.AddInstance` (`self.InstancedStaticMesh`) _returnvalue false))
  (`InstancedStaticMeshComponent.SetCustomDataValue` (`self.InstancedStaticMesh`) _returnvalue_4 0 2.0 false))